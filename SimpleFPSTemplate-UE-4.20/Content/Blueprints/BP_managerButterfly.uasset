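; Butterfly flock manager that gathers existing BP_butterfly actors at BeginPlay and spawns more at random offsets around the player.
; Tick applies a boids-style cohesion step (V1), setting each velocity toward the others' average position, adding it to the stored position and moving the actor.
; Separation (V2), velocity matching (V3) and the CheckPosition bounds flip are defined but never run, so only cohesion drives movement.
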(event `self.ReceiveBeginPlay`
  (bind _outactors (`GameplayStatics.GetAllActorsOfClass` "/Game/Blueprints/BP_butterfly.BP_butterfly_C"))
  (set `self.ButterflyArray` _outactors)
  (`self.Spawn`))

(event `self.ReceiveTick`
  (params (DeltaSeconds :type "Float (single-precision)"))
  (for (_array_element _array_index) (`self.ButterflyArray`)
    (bind _v1 (`self.V1` _array_element _array_index))
    (bind _returnvalue (+ _v1 (0.0 0.0 0.0) (0.0 0.0 0.0) (0.0 0.0 0.0)))
    (`KismetArrayLibrary.Array_Set` (`self.Velocity`) _array_index _returnvalue)
    (`KismetArrayLibrary.Array_Set` (`self.Position`) _array_index (+ _returnvalue (`|GetArrayItem` (`self.Position`) _array_index)))
    (`self.K2_SetActorTransform` (`|GetArrayItem` (`self.ButterflyArray`) _array_index) (`KismetMathLibrary.Conv_VectorToTransform` (`|GetArrayItem` (`self.Position`) _array_index)) false false)))

(fn `check position`
  (params (POSITION :type "Vector Structure") (INDEX :type Integer))
  (returns (VELOCITY :type "Vector Structure"))
  (bind _maxfloat (`self.MAXFLOAT`))
  (bind (_output_x _output_y _output_z) (`KismetMathLibrary.BreakVector` (`|GetArrayItem` (`self.Velocity`) INDEX)))
  (if (> (`KismetMathLibrary.Abs` POSITION_X) _maxfloat)
    (return (`KismetMathLibrary.MakeVector` (* _output_x -1.0) POSITION_Y POSITION_Z))
    (elif (> (`KismetMathLibrary.Abs` POSITION_Y) _maxfloat)
      (return (`KismetMathLibrary.MakeVector` POSITION_X (* _output_y -1.0) POSITION_Z))
      (elif (> (`KismetMathLibrary.Abs` POSITION_Z) _maxfloat)
        (return (`KismetMathLibrary.MakeVector` POSITION_X POSITION_Y (* _output_z -1.0)))
        (else
          (return (`KismetMathLibrary.MakeVector` _output_x _output_y _output_z)))))))

(fn `Spawn`
  (bind _position (`self.Position`))
  (bind _returnvalue (`self.GetTransform` (`GameplayStatics.GetPlayerCharacter` 0)))
  (for _ (range (+ (`self.MaxButterfly`) 1))
    (bind _returnvalue_2 (`KismetArrayLibrary.Array_Add` _position (`KismetMathLibrary.MakeVector` (+ (.x (.location _returnvalue)) (`KismetMathLibrary.RandomFloatInRange` -10.0 300.0)) (+ (.y (.location _returnvalue)) (`KismetMathLibrary.RandomFloatInRange` -10.0 300.0)) (+ (.z (.location _returnvalue)) (`KismetMathLibrary.RandomFloatInRange` -10.0 300.0)))))
    (bind _returnvalue_3 (`|SpawnActorFromClass` "/Game/Blueprints/BP_butterfly.BP_butterfly_C" (`KismetMathLibrary.MakeTransform` (`|GetArrayItem` _position _returnvalue_2) (.rotation _returnvalue)) "Undefined" "OverrideRootScale" null null))
    (`KismetArrayLibrary.Array_Add` (`self.ButterflyArray`) _returnvalue_3)
    (`KismetArrayLibrary.Array_Add` (`self.Velocity`) (`KismetMathLibrary.RandomUnitVector`))))

(fn `UserConstructionScript`)

(fn `V1`
  (params (Current :type "/Game/Blueprints/BP_butterfly Object Reference") (index :type Integer))
  (returns (v1 :type "Vector Structure"))
  (locals (PerceivedofCenterMasa :type "Vector Structure"))
  (set `local.PerceivedofCenterMasa` (0.0 0.0 0.0))
  (for (_ _array_index) (`self.ButterflyArray`)
    (if (!= index _array_index)
      (set `local.PerceivedofCenterMasa` (+ (`local.PerceivedofCenterMasa`) (`|GetArrayItem` (`self.Position`) _array_index)))))
  (set `local.PerceivedofCenterMasa` (/ (`local.PerceivedofCenterMasa`) (- (`self.MaxButterfly`) 1)))
  (return (/ (- (`local.PerceivedofCenterMasa`) (`|GetArrayItem` (`self.Position`) index)) 10000)))

(fn `V2`
  (params (Current :type "/Game/Blueprints/BP_butterfly Object Reference") (index :type Integer))
  (returns (v2 :type "Vector Structure"))
  (locals (PerceivedofCenterMasa :type "Vector Structure") (C :type "Vector Structure"))
  (bind _position (`self.Position`))
  (bind (_distanceinbetween_x _distanceinbetween_y _distanceinbetween_z) (`KismetMathLibrary.BreakVector` (`self.DistanceinBetween`)))
  (set `local.C` (0.0 0.0 0.0))
  (for (_ _array_index) (`self.ButterflyArray`)
    (if (!= index _array_index)
      (bind _returnvalue (- (`|GetArrayItem` _position _array_index) (`|GetArrayItem` _position index)))
      (bind (_returnvalue_x _returnvalue_y _returnvalue_z) (`KismetMathLibrary.BreakVector` (`KismetMathLibrary.Vector_GetAbs` _returnvalue)))
      (if (< _returnvalue_x _distanceinbetween_x)
        (if (< _returnvalue_y _distanceinbetween_y)
          (if (< _returnvalue_z _distanceinbetween_z)
            (set `local.C` (- (`local.C`) _returnvalue))
            (return (`local.C`))))))))

(fn `v3`
  (params (Current :type "/Game/Blueprints/BP_butterfly Object Reference") (index :type Integer))
  (returns (v3 :type "Vector Structure"))
  (locals (PerceivedofCenterMasa :type "Vector Structure") (PerceivedVelocity :type "Vector Structure"))
  (set `local.PerceivedVelocity` (0.0 0.0 0.0))
  (for (_ _array_index) (`self.ButterflyArray`)
    (if (!= index _array_index)
      (set `local.PerceivedVelocity` (+ (`local.PerceivedVelocity`) (`|GetArrayItem` (`self.Velocity`) _array_index)))))
  (set `local.PerceivedofCenterMasa` (/ (`local.PerceivedVelocity`) (- (`self.MaxButterfly`) 1)))
  (return (/ (- (`local.PerceivedVelocity`) (`|GetArrayItem` (`self.Velocity`) index)) 100)))