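; BoidManager is a flocking manager meant to configure and spawn boids, but its logic sits in unconnected paths, with BeginPlay and Tick empty.
; SetBoid copies steering weights, limits and an optional goal onto each boid.
; The unwired logic initializes placed boids and spawns more at timed intervals up to MaxBoids, above random navmesh points with randomized goal-seek weight.
; The spawn node has no class set.
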(event `self.ReceiveBeginPlay`)

(event `self.ReceiveTick`
  (params (DeltaSeconds :type "Float (single-precision)")))

(fn `Set Boid`
  (params (GoalSeekWeight :type "Float (double-precision)") (AlignmentWeight :type "Float (double-precision)") (CohesionWeight :type "Float (double-precision)") (SeperationWeight :type "Float (double-precision)") (MaxSpeed :type "Float (double-precision)") (MaxForce :type "Float (double-precision)") (NeighborhoodDist :type "Float (double-precision)") (DesiredSeperation :type "Float (double-precision)") (Boid :type "Object Object Reference") (`Boid Goal` :type "Actor Object Reference"))
  (`/Engine/EditorBlueprintResources/StandardMacros.IsValid` Boid
    (:`Is Valid`
      (`|ExecutionSequence`
        (:`then_0`
          (set `/Game/Blueprints/BoidManager.GoalSeekWeight` GoalSeekWeight Boid)
          (set `/Game/Blueprints/BoidManager.AlignmentWeight` AlignmentWeight Boid)
          (set `/Game/Blueprints/BoidManager.CohesionWeight` CohesionWeight Boid)
          (set `/Game/Blueprints/BoidManager.SeparationWeight` SeperationWeight Boid)
          (set `/Game/Blueprints/BoidManager.MaxSpeed` MaxSpeed Boid)
          (set `/Game/Blueprints/BoidManager.MaxForce` MaxForce Boid)
          (set `/Game/Blueprints/BoidManager.NeighborhoodDist` NeighborhoodDist Boid)
          (set `/Game/Blueprints/BoidManager.DesiredSeparation` DesiredSeperation Boid))
        (:`then_1`
          (`/Engine/EditorBlueprintResources/StandardMacros.IsValid` `Boid Goal`
            (:`Is Valid`
              (set `/Game/Blueprints/BoidManager.Goal` `Boid Goal` Boid))))))))

(fn `UserConstructionScript`)